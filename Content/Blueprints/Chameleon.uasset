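; Touchable chameleon actor that changes to the color synthesized in the master widget and submits it to the game mode's color check.
; A touch plays an optional sound, maps the finger's hit point to material X/Y, and sets previous and new color parameters.
; A timeline animates the material's Radius from that origin, then calls CheckColor and re-enables touch.
; Touches are ignored mid-transition or during game over.
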(event EventBeginPlay
  (bind _asgi (Utilities|Casting|CastToGI (Game|GetGameInstance)))
  (Variables|Default|Set%20GI _asgi))

(event EventActorOnInputTouchBegin
  (params (FingerIndex :type ETouchIndex%20Enum :default "Touch1"))
  (bind _chameleonmesh (Variables|Default|GetChameleonMesh))
  (bind _aspc_game (Utilities|Casting|CastToPC_Game (Game|GetPlayerController 0))
    (:then
      (if (not (or (Variables|Default|GetIsTouch) (Variables|/Game/Blueprints/UI/WBP_Master.WBP_Master_C|GetbGameOverState (Variables|/Game/Blueprints/Framework/PC_Game.PC_Game_C|GetMasterWidget _aspc_game))))
        (Variables|Default|SetIsTouch true :!label _label)
        (CallFunction|PlaySound)
        (Utilities|SetColorChangeOrigin)
        (Rendering|Material|SetVectorParameterValueonMaterials _chameleonmesh "PreviousColor" (Variables|Default|GetBodyColor))
        (bind _result (|CollapseGraph))
        (bind _output_get (Variables|Default|SetBodyColor _result))
        (Rendering|Material|SetVectorParameterValueonMaterials _chameleonmesh "NewColor" _output_get)
        (bind _radius (Timeline|Timeline PlayFromStart)
          (:Update
            (Rendering|Material|SetScalarParameterValueonMaterials _chameleonmesh "Radius" _radius))
          (:Finished
            (bind _asgm_game (Utilities|Casting|CastToGM_Game (Game|GetGameMode)))
            (Default|CheckColor _asgm_game (Variables|Default|GetBodyColor))
            (Variables|Default|SetIsTouch false)
            (Class|WidgetBlueprintLibrary|CancelDragDrop)))))
    (:CastFailed
      (if (not (Variables|Default|GetIsTouch))
        (goto _label)))))

(fn ConstructionScript
  (bind _output_get (Variables|Default|SetBodyColor (Math|Vector|MakeVector 0.062662 0.320833 0.0)))
  (Rendering|Material|SetVectorParameterValueonMaterials (Variables|Default|GetChameleonMesh) "PreviousColor" _output_get)
  (Rendering|Material|SetScalarParameterValueonMaterials (Variables|Default|GetChameleonMesh) "Radius" 0.0))

(fn PlaySound
  (bind __gi (Variables|Default|Get%20GI)
    (:then
      (if (Variables|/Game/Blueprints/Framework/GI.GI_C|GetPlaySound __gi)
        (Audio|PlaySound2D "/Game/Sound/Effect/Retro_PickUp_Coin_04.Retro_PickUp_Coin_04" 1.0 1.0 0.0 0 0 false)))
    (:else
      _))
  (return))