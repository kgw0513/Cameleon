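; Cameleon is a touch-reactive plane actor that changes to a random color, spreading from the touched point.
; On touch, it converts the finger trace's world X/Y impact into material coordinates, assuming a 100-unit plane centered on the world origin.
; It passes the previous and new colors to the material, then a timeline animates the Radius parameter.
; The construction script sets a fixed starting color and zero radius.
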(event EventActorOnInputTouchBegin
  (params (FingerIndex :type ETouchIndex%20Enum :default "Touch1"))
  (bind _returnvalue (Game|GetPlayerController 0))
  (bind _plane (Variables|Default|GetPlane))
  (bind _hitresult (Class|PlayerController|GetHitResultUnderFingerbyChannel _returnvalue "Touch1" "TraceTypeQuery1" true))
  (bind _impactpoint (Collision|BreakHitResult _hitresult))
  (bind (_x _y) (Math|Vector|BreakVector _impactpoint))
  (Rendering|Material|SetScalarParameterValueonMaterials (Variables|Default|GetPlane) "X" (/ (+ _x 5e+01) 1e+02))
  (Rendering|Material|SetScalarParameterValueonMaterials (Variables|Default|GetPlane) "Y" (/ (+ _y 5e+01) 1e+02))
  (Rendering|Material|SetVectorParameterValueonMaterials _plane "PreviousColor" (Variables|Default|GetNewVar))
  (bind _output_get (Variables|Default|SetNewVar (Math|Vector|MakeVector (Math|Random|RandomFloatinRange 0.0 1.0) (Math|Random|RandomFloatinRange 0.0 1.0) (Math|Random|RandomFloatinRange 0.0 1.0))))
  (Rendering|Material|SetVectorParameterValueonMaterials (Variables|Default|GetPlane) "NewColor" _output_get)
  (bind _radius (Timeline|Timeline PlayFromStart)
    (:Update
      (Rendering|Material|SetScalarParameterValueonMaterials _plane "Radius" _radius))))

(fn ConstructionScript
  (bind _output_get (Variables|Default|SetNewVar (Math|Vector|MakeVector 0.062662 0.320833 0.0)))
  (Rendering|Material|SetVectorParameterValueonMaterials (Variables|Default|GetPlane) "PreviousColor" _output_get)
  (Rendering|Material|SetScalarParameterValueonMaterials (Variables|Default|GetPlane) "Radius" 0.0))