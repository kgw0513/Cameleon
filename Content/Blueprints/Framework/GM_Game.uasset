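; Game mode for a color-matching game that builds each match's background color and tube color array.
; BeginPlay caches the first StaticMeshActor found as the background mesh, which PrepareMatch tints randomly.
; PrepareMatch derives two tube colors per channel so their sum minus one equals the background, then adds three random decoys.
; Decoys regenerate recursively when IsNearlyEqualToActualColor flags them.
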(event Custom|SetBackgroundReference
  (bind _outactors (Actor|GetAllActorsOfClass "/Script/Engine.StaticMeshActor"))
  (Variables|Default|SetBackgroundMesh (Variables|/Script/Engine.StaticMeshActor|GetStaticMeshComponent (Utilities|Array|Get(acopy) _outactors))))

(event EventBeginPlay
  (CallFunction|SetBackgroundReference))

(fn ConstructionScript)

(fn MakeBackgroundColor
  (bind _output_get (Variables|Default|SetBackgroundColor (Math|Vector|MakeVector (Math|Random|RandomFloatinRange 0.0 1.0) (Math|Random|RandomFloatinRange 0.0 1.0) (Math|Random|RandomFloatinRange 0.0 1.0))))
  (Rendering|Material|SetVectorParameterValueonMaterials (Variables|Default|GetBackgroundMesh) "Color" _output_get)
  (return (Variables|Default|GetBackgroundColor)))

(fn MakeTubeColors
  (params (BackGroundColor :type Vector))
  (bind _colors (Variables|Default|GetColors))
  (Utilities|FlowControl|Sequence
    (:then_0
      (bind (_returna _returnb) (CallFunction|DivideFloatforDesiredColor (.x BackGroundColor))))
    (:then_1
      (bind (_returna_2 _returnb_2) (CallFunction|DivideFloatforDesiredColor (.y BackGroundColor))))
    (:then_2
      (bind (_returna_3 _returnb_3) (CallFunction|DivideFloatforDesiredColor (.z BackGroundColor)))
      (bind _output_get (Variables|Default|SetTubeColorA (Math|Vector|MakeVector _returna _returna_2 _returna_3)))
      (Utilities|Array|SetArrayElem _colors 0 _output_get true)
      (bind _output_get_2 (Variables|Default|SetTubeColorB (Math|Vector|MakeVector _returnb _returnb_2 _returnb_3)))
      (Utilities|Array|SetArrayElem _colors 1 _output_get_2 true)
      (return))))

(fn DivideFloatforDesiredColor
  (params (FloatFromSource :type Float%20%28double-precision%29))
  (bind _output_get (LocalVariables|SetRemColor (Math|Random|RandomFloatinRange FloatFromSource 1.0)))
  (return _output_get (Utilities|Operators|Subtract FloatFromSource _output_get -1.0)))

(fn SetFakeColors
  (for _index (range 2 4)
    (bind _returnvector (CallFunction|GenerateDesiredFakeColor))
    (Utilities|Array|SetArrayElem (Variables|Default|GetColors) _index _returnvector true)))

(fn GenerateDesiredFakeColor
  (bind _output_get (LocalVariables|SetRandomlyGeneratedFakeColor (Math|Vector|MakeVector (Math|Random|RandomFloatinRange 0.0 1.0) (Math|Random|RandomFloatinRange 0.0 1.0) (Math|Random|RandomFloatinRange 0.0 1.0))))
  (if (Utilities|IsNearlyEqualtoActualColor _output_get)
    (bind _returnvector (CallFunction|GenerateDesiredFakeColor))
    (return _returnvector)
    (else
      (return _output_get))))

(fn PrepareMatch
  (bind _returnvalue (CallFunction|MakeBackgroundColor))
  (CallFunction|MakeTubeColors _returnvalue)
  (CallFunction|SetFakeColors)
  (return (Variables|Default|GetColors)))